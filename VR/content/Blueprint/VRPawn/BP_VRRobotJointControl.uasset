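; VR robot joint control that turns left-stick values into jog service calls on a six-axis robot.
; Tick runs an edge-triggered state check with a deadzone: up and down cycle the selected axis, left and right set direction.
; Left or right unpauses a looping timer that repeatedly sends start-jog calls through the robot manager.
; Each state change, including release to neutral, first pauses that timer and sends a stop-jog call.
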(event `self.ReceiveBeginPlay`
  (bind _returnvalue (`KismetSystemLibrary.K2_SetTimerDelegate` (delegate `StartJogging`) (`self.JoggingInteral`) true))
  (bind _output_get (set `self.JoggingTimer` _returnvalue))
  (`KismetSystemLibrary.K2_PauseTimerHandle` _output_get))

(event `StartJogging`
  (`ServiceCallStartJogging.ServiceCallStartJogging` (`NexDroidRobotManager.GetInstance`) (`self.CurrentJoggingAxis`) (`self.CurrentJoggingDir`)))

(event `StopJogging`
  (`KismetSystemLibrary.K2_PauseTimerHandle` (`self.JoggingTimer`))
  (`ServiceCallStopJogging.ServiceCallStopJogging` (`NexDroidRobotManager.GetInstance`) (`self.CurrentJoggingAxis`)))

(event `self.ReceiveTick`
  (params (DeltaSeconds :type "Float (single-precision)"))
  (bind _processed (`self.UpdateUp`))
  (if (not _processed)
    (bind _processed_2 (`self.UpdateDown`))
    (if (not _processed_2)
      (bind _processed_3 (`self.UpdateLeft`))
      (if (not _processed_3)
        (bind _processed_4 (`self.UpdateRight`))
        (if (not _processed_4)
          (`self.UpdateOther`))))))

(fn `IsOnlyXValueGraterThanDeadzone`
  (returns (ReturnValue :type Boolean))
  (return (and (`self.IsValueGraterThanDeadzone` (`self.MovementAxisLeftX`)) (not (`self.IsValueGraterThanDeadzone` (`self.MovementAxisLeftY`))))))

(fn `IsOnlyYValueGraterThanDeadzone`
  (returns (ReturnValue :type Boolean))
  (return (and (`self.IsValueGraterThanDeadzone` (`self.MovementAxisLeftY`)) (not (`self.IsValueGraterThanDeadzone` (`self.MovementAxisLeftX`))))))

(fn `IsValueGraterThanDeadzone`
  (params (Value :type "Float (double-precision)"))
  (returns (ReturnValue :type Boolean))
  (return (>= (`KismetMathLibrary.Abs` Value) 0.7)))

(fn `SetMovementAxisLeftValue`
  (params (X :type "Float (double-precision)") (Y :type "Float (double-precision)"))
  (set `self.MovementAxisLeftX` X)
  (set `self.MovementAxisLeftY` Y))

(fn `UpdateDown`
  (returns (Processed :type Boolean))
  (if (and (`self.IsOnlyYValueGraterThanDeadzone`) (< (`self.MovementAxisLeftY`) 0.0) (`|EnumInequality` (`self.CurrentVRAxisState`) "NewEnumerator1"))
    (`|ExecutionSequence`
      (:`then_0`
        (`self.StopJogging`))
      (:`then_1`
        (set `self.CurrentVRAxisState` "NewEnumerator1"))
      (:`then_2`
        (switch `ERobotAxis` (`self.CurrentJoggingAxis`)
          (:`Axis1`
            (set `self.CurrentJoggingAxis` "Axis2"))
          (:`Axis2`
            (set `self.CurrentJoggingAxis` "Axis3"))
          (:`Axis3`
            (set `self.CurrentJoggingAxis` "Axis4"))
          (:`Axis4`
            (set `self.CurrentJoggingAxis` "Axis5"))
          (:`Axis5`
            (set `self.CurrentJoggingAxis` "Axis6"))
          (:`Axis6`
            (set `self.CurrentJoggingAxis` "Axis1"))))
      (:`then_3`
        (return true)))
    (else
      (return false))))

(fn `UpdateLeft`
  (returns (Processed :type Boolean))
  (if (and (`self.IsOnlyXValueGraterThanDeadzone`) (< (`self.MovementAxisLeftX`) 0.0) (`|EnumInequality` (`self.CurrentVRAxisState`) "NewEnumerator2"))
    (`|ExecutionSequence`
      (:`then_0`
        (`self.StopJogging`))
      (:`then_1`
        (set `self.CurrentVRAxisState` "NewEnumerator2"))
      (:`then_2`
        (set `self.CurrentJoggingDir` false)
        (`KismetSystemLibrary.K2_UnPauseTimerHandle` (`self.JoggingTimer`)))
      (:`then_3`
        (return true)))
    (else
      (return false))))

(fn `UpdateOther`
  (returns (Processed :type Boolean))
  (if (and (not (`self.IsOnlyXValueGraterThanDeadzone`)) (not (`self.IsOnlyYValueGraterThanDeadzone`)) (`|EnumInequality` (`self.CurrentVRAxisState`) "NewEnumerator4"))
    (`|ExecutionSequence`
      (:`then_0`
        (`self.StopJogging`))
      (:`then_1`
        (set `self.CurrentVRAxisState` "NewEnumerator4"))
      (:`then_2`
        (return true)))
    (else
      (return false))))

(fn `UpdateRight`
  (returns (Processed :type Boolean))
  (if (and (`self.IsOnlyXValueGraterThanDeadzone`) (> (`self.MovementAxisLeftX`) 0.0) (`|EnumInequality` (`self.CurrentVRAxisState`) "NewEnumerator3"))
    (`|ExecutionSequence`
      (:`then_0`
        (`self.StopJogging`))
      (:`then_1`
        (set `self.CurrentVRAxisState` "NewEnumerator3"))
      (:`then_2`
        (set `self.CurrentJoggingDir` true)
        (`KismetSystemLibrary.K2_UnPauseTimerHandle` (`self.JoggingTimer`)))
      (:`then_3`
        (return true)))
    (else
      (return false))))

(fn `UpdateUp`
  (returns (Processed :type Boolean))
  (if (and (`self.IsOnlyYValueGraterThanDeadzone`) (> (`self.MovementAxisLeftY`) 0.0) (`|EnumInequality` (`self.CurrentVRAxisState`) "NewEnumerator0"))
    (`|ExecutionSequence`
      (:`then_0`
        (`self.StopJogging`))
      (:`then_1`
        (set `self.CurrentVRAxisState` "NewEnumerator0"))
      (:`then_2`
        (switch `ERobotAxis` (`self.CurrentJoggingAxis`)
          (:`Axis1`
            (set `self.CurrentJoggingAxis` "Axis6"))
          (:`Axis2`
            (set `self.CurrentJoggingAxis` "Axis1"))
          (:`Axis3`
            (set `self.CurrentJoggingAxis` "Axis2"))
          (:`Axis4`
            (set `self.CurrentJoggingAxis` "Axis3"))
          (:`Axis5`
            (set `self.CurrentJoggingAxis` "Axis4"))
          (:`Axis6`
            (set `self.CurrentJoggingAxis` "Axis5"))))
      (:`then_3`
        (return true)))
    (else
      (return false))))