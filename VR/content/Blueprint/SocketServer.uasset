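; SocketServer is a TCP server that sends motion transforms and controller key input to a connected client as JSON.
; On BeginPlay it starts an ObjectDeliverer manager on port 8000 with fixed-length 180 packets and a UTF-8 string delivery box.
; SendTransform and SendKey serialize FinalTransform or key/axis values into structs and send them through that box.
; Connection changes, received strings and sent payloads are printed on screen.
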(event `self.ReceiveBeginPlay`
  (`|ExecutionSequence`
    (:`then_0`
      ;[1 1 1] 创建DeliverManager
      (bind _output_get (set `self.Deliverer` (`ObjectDelivererManager.CreateObjectDelivererManager` true)))
      (add `ObjectDelivererManager.Connected` _output_get (delegate `OnConnected`))
      (add `ObjectDelivererManager.Disconnected` _output_get (delegate `OnDisconnected`)))
    (:`then_1`
      ;[1 1 1] 创建DeliveryBox
      (bind _output_get_2 (set `self.DelilveryBoxString` (`DeliveryBoxFactory.CreateUtf8StringDeliveryBox`)))
      (add `Utf8StringDeliveryBox.Received` _output_get_2 (delegate `OnReceived`)))
    (:`then_2`
      ;[1 1 1] 打开TCPIP端口
      (`ObjectDelivererManager.Start` (`self.Deliverer`) (`ProtocolFactory.CreateProtocolTcpIpServer` 8000) (`PacketRuleFactory.CreatePacketRuleFixedLength` 180) (`self.DelilveryBoxString`)))))

(event `OnConnected`
  (params (ClientSocket :type "ObjectDelivererProtocol Object Reference"))
  ;[1 1 1] 创建DeliverManager
  (set `self.Client Socket` ClientSocket)
  (`KismetSystemLibrary.PrintString` "Connected(Client)" true true (struct :`G` 0.66 :`B` 1.0 :`A` 1.0) 10.0))

(event `OnDisconnected`
  (params (ClientSocket :type "ObjectDelivererProtocol Object Reference"))
  ;[1 1 1] 创建DeliverManager
  (`KismetSystemLibrary.PrintString` "Disconnected(Client)" true true (struct :`R` 1.0 :`A` 1.0) 10.0))

(event `OnReceived`
  (params (ReceivedString :type String) (FromObject :type "ObjectDelivererProtocol Object Reference"))
  ;[1 1 1] 创建DeliveryBox
  (`KismetSystemLibrary.PrintString` ReceivedString))

(event `SendTransform`
  (params (who :type String) (FinalTransform :type "Transform Structure"))
  ;[1 1 1] 发送体感数据
  (bind _returnvalue (`|JsonSerialize` (make `/Game/Blueprint/TransformStruct` who (.x (.location FinalTransform)) (.y (.location FinalTransform)) (.z (.location FinalTransform)) (.roll (.rotation FinalTransform)) (.pitch (.rotation FinalTransform)) (.yaw (.rotation FinalTransform)))))
  (`Utf8StringDeliveryBox.Send` (`self.DelilveryBoxString`) _returnvalue)
  (`KismetSystemLibrary.PrintString` _returnvalue true true (struct :`G` 0.66 :`B` 1.0 :`A` 1.0) 5.0))

(event `SendKey`
  (params (Key :type String) (AxisValue :type "Float (double-precision)"))
  ;[1 1 1] 发送手柄按键
  (bind _returnvalue (`|JsonSerialize` (make `/Game/Blueprint/KeyStruct` "key" Key AxisValue)))
  (`Utf8StringDeliveryBox.Send` (`self.DelilveryBoxString`) _returnvalue)
  (`KismetSystemLibrary.PrintString` _returnvalue true true (struct :`R` 0.042944 :`G` 1.0 :`A` 1.0)))

(fn `UserConstructionScript`)