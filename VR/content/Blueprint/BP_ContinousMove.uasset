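; Continuous motion-control actor that streams left and right controller poses to a SocketServer, apparently to drive robot end effectors.
; Initialize events set each hand's zero point and enable movement; Start and Stop events spawn and destroy a ControllerIndicator hint model.
; A delayed Tick snaps hints to followed components, converts their zero-relative poses to backend axes by swapping and negating, then sends them.
; The movement-threshold check exists but is unconnected.
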(event `InitializeTransformLeft`
  (params (`Follow Scene Component` :type "SceneComponent Object Reference"))
  (bind _returnvalue (`SceneComponent.K2_GetComponentToWorld` `Follow Scene Component`))
  ;[1 1 1] 重置坐标零位为当前位置（左手）
  (`|ExecutionSequence`
    (:`then_0`
      (`self.SetActorHiddenInGame` (`self.BaseTransformLeft`) false))
    (:`then_1`
      (set `self.PositionOffset` (0.0 0.0 0.0))
      (`self.K2_SetActorTransform` (`self.BaseTransformLeft`) _returnvalue false false)
      (bind _output_get (set `self.InitializedZeroPointLeft` _returnvalue))
      (set `self.HintModelLastTargetTransformLeft` _output_get)
      (`KismetSystemLibrary.PrintString` (`KismetStringLibrary.Conv_TransformToString` _output_get) true true (struct :`R` 1.0 :`G` 0.226286 :`B` 0.827676 :`A` 1.0) 10.0))
    (:`then_2`
      (`/Engine/EditorBlueprintResources/StandardMacros.DoOnce` false
        (:`Completed`
          (set `self.MovementActivatedLeft` true))))))

(event `InitializeTransformRight`
  (params (`Follow Scene Component` :type "SceneComponent Object Reference"))
  (bind _returnvalue (`SceneComponent.K2_GetComponentToWorld` `Follow Scene Component`))
  ;[1 1 1] 重置坐标零位为当前位置（右手）
  (`|ExecutionSequence`
    (:`then_0`
      (`self.SetActorHiddenInGame` (`self.BaseTransformRight`) false))
    (:`then_1`
      (set `self.PositionOffset` (0.0 0.0 0.0))
      (`self.K2_SetActorTransform` (`self.BaseTransformRight`) _returnvalue false false)
      (bind _output_get (set `self.InitializedZeroPointRight` _returnvalue))
      (set `self.HintModelLastTargetTransformRight` _output_get)
      (`KismetSystemLibrary.PrintString` (`KismetStringLibrary.Conv_TransformToString` _output_get) true true (struct :`R` 1.0 :`G` 0.429057 :`B` 0.07128 :`A` 1.0) 10.0))
    (:`then_2`
      (`/Engine/EditorBlueprintResources/StandardMacros.DoOnce` false
        (:`Completed`
          (set `self.MovementActivatedRight` true))))))

(event `self.ReceiveBeginPlay`
  ;[1 1 1] 开始时，获取并保存初始位置指示器模型
  (bind _outactors (`GameplayStatics.GetAllActorsOfClass` "/Game/Blueprint/BaseModelTransform.BaseModelTransform_C"))
  (set `self.BaseTransformLeft` (`|GetArrayItem` _outactors))
  (set `self.BaseTransformRight` (`|GetArrayItem` _outactors 1))
  (bind _returnvalue (`GameplayStatics.GetActorOfClass` "/Game/Blueprint/SocketServer.SocketServer_C"))
  (set `self.SocketServer` _returnvalue))

(event `StopContinousMoveRight`
  (bind _robotendhintmodelright (`self.RobotEndHintModelRight`))
  ;[1 1 1] 销毁hint模型
  (`/Engine/EditorBlueprintResources/StandardMacros.IsValid` _robotendhintmodelright
    (:`Is Valid`
      (`self.K2_DestroyActor` _robotendhintmodelright)
      ;[1 1 1] 记录上次移动结束位置
      (set `self.HintModelLastTargetTransformRight` (`SceneComponent.K2_GetComponentToWorld` (`Actor.RootComponent` _robotendhintmodelright)))
      ;[1 1 1] 将跟随组件置空
      (set `self.FollowCompRight` null)
      (`KismetSystemLibrary.PrintString` (`KismetStringLibrary.Conv_TransformToString` (`self.FinalTransformRight`)) true true (struct :`R` 1.0 :`G` 0.407399 :`A` 1.0) 10.0))))

(event `StopContinuousMoveLeft`
  (bind _robotendhintmodelleft (`self.RobotEndHintModelLeft`))
  ;[1 1 1] 左手，同上
  (`/Engine/EditorBlueprintResources/StandardMacros.IsValid` _robotendhintmodelleft
    (:`Is Valid`
      (`self.K2_DestroyActor` _robotendhintmodelleft)
      (set `self.HintModelLastTargetTransformLeft` (`SceneComponent.K2_GetComponentToWorld` (`Actor.RootComponent` _robotendhintmodelleft)))
      (set `self.FollowCompLeft` null)
      (`KismetSystemLibrary.PrintString` (`KismetStringLibrary.Conv_TransformToString` (`self.FinalTransformLeft`)) true true (struct :`R` 1.0 :`G` 0.093271 :`B` 0.73814 :`A` 1.0) 10.0))))

(event `StartContinousMoveRight`
  (params (FollowSceneComponent :type "SceneComponent Object Reference"))
  (if (`self.MovementActivatedRight`)
    (bind _output_get (set `self.FollowCompRight` FollowSceneComponent))
    ;[1 1 1] 记录此时follow组件的transform
    (bind _output_get_2 (set `self.FollowCompRightTransformWhenStart` (`SceneComponent.K2_GetComponentToWorld` _output_get)))
    ;[1 1 1] 在对应位置生成末端hint模型
    (bind _returnvalue (`|SpawnActorFromClass` "/Game/Blueprint/ControllerIndicator.ControllerIndicator_C" _output_get_2 "AlwaysSpawn" "OverrideRootScale" null null))
    (set `self.RobotEndHintModelRight` _returnvalue)
    (else
      (`KismetSystemLibrary.PrintString` "Press\"B\" to start motion control(Right)" true true (struct :`R` 1.0 :`B` 0.016047 :`A` 1.0) 10.0))))

(event `StartContinousMoveLeft`
  (params (FollowSceneComponent :type "SceneComponent Object Reference"))
  ;[1 1 1] 左手体感，同上
  (if (`self.MovementActivatedLeft`)
    (bind _output_get (set `self.FollowCompLeft` FollowSceneComponent))
    (bind _output_get_2 (set `self.FollowCompLeftTransformWhenStart` (`SceneComponent.K2_GetComponentToWorld` _output_get)))
    (bind _returnvalue (`|SpawnActorFromClass` "/Game/Blueprint/ControllerIndicator.ControllerIndicator_C" _output_get_2 "AlwaysSpawn" "OverrideRootScale" null null))
    (set `self.RobotEndHintModelLeft` _returnvalue)
    (else
      (`KismetSystemLibrary.PrintString` "Press\"Y\" to start motion control(Left)" true true (struct :`R` 1.0 :`B` 0.016047 :`A` 1.0) 10.0))))

(event `self.ReceiveTick`
  (params (DeltaSeconds :type "Float (single-precision)"))
  (bind _robotendhintmodelright (`self.RobotEndHintModelRight`))
  (bind _robotendhintmodelleft (`self.RobotEndHintModelLeft`))
  (`KismetSystemLibrary.Delay` 0.03)
  (`|ExecutionSequence`
    (:`then_0`
      (`/Engine/EditorBlueprintResources/StandardMacros.IsValid` _robotendhintmodelright
        (:`Is Valid`
          (`self.UpdateGestureControlHintModel` _robotendhintmodelright (`self.FollowCompRight`))
          ;[1 1 1] 应后端要求进行坐标转换：对调X、Y轴，R、P、Y对应X、Y、Z，全右手系
          (bind _output_get (set `self.FinalTransformRight` (`KismetMathLibrary.MakeTransform` (`KismetMathLibrary.MakeVector` (* (.y (.location (`self.GetGestureControlRelativeTransform` (`self.RobotEndHintModelRight`) (`self.InitializedZeroPointRight`)))) -1.0) (* (.x (.location (`self.GetGestureControlRelativeTransform` (`self.RobotEndHintModelRight`) (`self.InitializedZeroPointRight`)))) -1.0) (.z (.location (`self.GetGestureControlRelativeTransform` (`self.RobotEndHintModelRight`) (`self.InitializedZeroPointRight`))))) (`KismetMathLibrary.MakeRotator` (* (.pitch (.rotation (`self.GetGestureControlRelativeTransform` (`self.RobotEndHintModelRight`) (`self.InitializedZeroPointRight`)))) -1.0) (* (.roll (.rotation (`self.GetGestureControlRelativeTransform` (`self.RobotEndHintModelRight`) (`self.InitializedZeroPointRight`)))) -1.0) (* (.yaw (.rotation (`self.GetGestureControlRelativeTransform` (`self.RobotEndHintModelRight`) (`self.InitializedZeroPointRight`)))) -1.0)))))
          (`/Game/Blueprint/SocketServer.SendTransform` (`self.SocketServer`) "right" _output_get))))
    (:`then_1`
      (`/Engine/EditorBlueprintResources/StandardMacros.IsValid` _robotendhintmodelleft
        (:`Is Valid`
          (`self.UpdateGestureControlHintModel` _robotendhintmodelleft (`self.FollowCompLeft`))
          (bind _output_get_2 (set `self.FinalTransformLeft` (`KismetMathLibrary.MakeTransform` (`KismetMathLibrary.MakeVector` (* (.y (.location (`self.GetGestureControlRelativeTransform` (`self.RobotEndHintModelLeft`) (`self.InitializedZeroPointLeft`)))) -1.0) (* (.x (.location (`self.GetGestureControlRelativeTransform` (`self.RobotEndHintModelLeft`) (`self.InitializedZeroPointLeft`)))) -1.0) (.z (.location (`self.GetGestureControlRelativeTransform` (`self.RobotEndHintModelLeft`) (`self.InitializedZeroPointLeft`))))) (`KismetMathLibrary.MakeRotator` (* (.pitch (.rotation (`self.GetGestureControlRelativeTransform` (`self.RobotEndHintModelLeft`) (`self.InitializedZeroPointLeft`)))) -1.0) (* (.roll (.rotation (`self.GetGestureControlRelativeTransform` (`self.RobotEndHintModelLeft`) (`self.InitializedZeroPointLeft`)))) -1.0) (* (.yaw (.rotation (`self.GetGestureControlRelativeTransform` (`self.RobotEndHintModelLeft`) (`self.InitializedZeroPointLeft`)))) -1.0)))))
          (`/Game/Blueprint/SocketServer.SendTransform` (`self.SocketServer`) "left" _output_get_2))))))

(fn `CheckMoveTargetTransform`
  (params (HintModel :type "Actor Object Reference") (LastTransform :type "Transform Structure"))
  (returns (NeedMove :type Boolean) (NewTransform :type "Transform Structure"))
  (locals (RobotAxisRefLocalLocation :type "Vector Structure" :default (0.0 0.0 0.0)))
  (`/Engine/EditorBlueprintResources/StandardMacros.IsValid` HintModel
    (:`Is Valid`
      (if (and (== (.location (`self.GetTransform` HintModel)) (.location LastTransform) :`ErrorTolerance` (`self.MoveTargetLocationThreshold`)) (== (.rotation (`self.GetTransform` HintModel)) (.rotation LastTransform) :`ErrorTolerance` (`self.MoveTargetRotationThreshold`)))
        ;[1 1 1] 变化小，不需要移动
        (return false LastTransform)
        (else
          ;[1 1 1] 变化大，需要移动
          (return true (`self.GetTransform` HintModel)))))))

(fn `GetGestureControlRelativeTransform`
  (params (HintModel :type "Actor Object Reference") (RelativePoint :type "Transform Structure"))
  (returns (RelativeTransform :type "Transform Structure"))
  (locals (RobotAxisRefLocalLocation :type "Vector Structure" :default (0.0 0.0 0.0)))
  (bind (_returnvalue_location _returnvalue_rotation) (`KismetMathLibrary.BreakTransform` (`KismetMathLibrary.MakeRelativeTransform` (`SceneComponent.K2_GetComponentToWorld` (`Actor.RootComponent` HintModel)) RelativePoint)))
  ;[1 1 1] 将右手柄移动的向量，转换到新原点的相对坐标
  (return (`KismetMathLibrary.MakeTransform` _returnvalue_location _returnvalue_rotation)))

(fn `TestStart`
  (`self.StartContinousMoveRight` (`self.DefaultSceneRoot`)))

(fn `TestStop`
  (`self.StopContinousMoveRight`))

(fn `UpdateGestureControlHintModel`
  (params (HintModel :type "Actor Object Reference") (FollowComp :type "SceneComponent Object Reference"))
  (locals (RobotAxisRefLocalLocation :type "Vector Structure" :default (0.0 0.0 0.0)))
  (bind (_returnvalue_location _returnvalue_rotation) (`KismetMathLibrary.BreakTransform` (`SceneComponent.K2_GetComponentToWorld` FollowComp)))
  (`/Engine/EditorBlueprintResources/StandardMacros.IsValid` HintModel
    (:`Is Valid`
      (`self.K2_SetActorLocationAndRotation` HintModel _returnvalue_location _returnvalue_rotation false false)
      (return))))

(fn `UserConstructionScript`)