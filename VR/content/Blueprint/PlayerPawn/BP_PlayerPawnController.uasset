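; Player controller that creates the main UI canvas, switches between orbit and third-person pawns, and drives robot test commands from number keys.
; On init it starts a looping timer that publishes the controlled pawn's transform through a singleton only when that pawn type is visible.
; Debug keys call RobotMgr services for joint or XYZ moves, continuous-motion mode toggling and a queued NRC command sequence, with several alternative queues left unwired.
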(event `Key|One`
  (params (Key :type "Key Structure"))
  (:`Released`
    (`self.EnterOrbit` false)))

(event `Key|Two`
  (params (Key :type "Key Structure"))
  ;[1 1 1] PC端只有在自己测试时，才可触发第三人称pawn
  (:`Released`
    (`self.EnterThird`)))

(event `PublishPawnData`
  (bind _returnvalue (`self.K2_GetPawn`))
  (switch `EPawnVisibilityType` (`BlueprintMapLibrary.Map_Find` (`self.PawnVisibilityMap`) (`self.CurrentPawnType`))
    (:`Visible`
      (`NexDroidRobotManager.PublishPawnData` (`NexDroidRobotManager.GetInstance`) "Visible" (`self.K2_GetActorLocation` _returnvalue) (`self.K2_GetActorRotation` _returnvalue)))))

(event `self.OnInit`
  (`|ExecutionSequence`
    (:`then_0`
      (`KismetSystemLibrary.K2_SetTimerDelegate` (delegate `PublishPawnData`) (`self.PublishPawnDataInterval`) true))
    (:`then_1`
      (bind _returnvalue (`|CreateWidget` "/Game/Blueprint/UI/WBP_MainCanvas.WBP_MainCanvas_C" self))
      (`UserWidget.AddToViewport` _returnvalue 0))))

(event `Key|Three`
  (params (Key :type "Key Structure"))
  (:`Released`
    (`ServiceCallRobotMovj.ServiceCallRobotMovj` (`NexDroidRobotManager.GetInstance`) (`|MakeArray` 0.0 0.0 0.0 0.0 0.0 0.0 :!type "Float (single-precision)") 100 "Joint")))

(event `Key|Four`
  (params (Key :type "Key Structure"))
  (:`Released`
    (`ServiceCallRobotMovj.ServiceCallRobotMovj` (`NexDroidRobotManager.GetInstance`) (`|MakeArray` 180.0 0.0 0.0 0.0 0.0 0.0 :!type "Float (single-precision)") 100 "XYZ")))

(event `Key|Five`
  (params (Key :type "Key Structure"))
  (:`Released`
    (`ServiceCallContinuousMotionMode.ServiceCallContinuousMotionMode` (`NexDroidRobotManager.GetInstance`) true
      (:`then`
        (`KismetSystemLibrary.PrintString` "开启连续运动模式"))
      (:`OnSuccess`
        (`KismetSystemLibrary.PrintString` "开启连续运动模式 success")))))

(event `Key|Six`
  (params (Key :type "Key Structure"))
  (:`Released`
    (`ServiceCallContinuousMotionMode.ServiceCallContinuousMotionMode` (`NexDroidRobotManager.GetInstance`)
      (:`then`
        (`KismetSystemLibrary.PrintString` "关闭连续运动模式"))
      (:`OnSuccess`
        (`KismetSystemLibrary.PrintString` "关闭连续运动模式 success")))))

(event `Key|Seven`
  (params (Key :type "Key Structure"))
  (:`Released`
    (`ServiceCallSendContinuousMotionQueue.ServiceCallSendContinuousMotionQueue` (`NexDroidRobotManager.GetInstance`) (`|MakeArray` (make `NrcCmd` 1 100.0 30.0 30.0 1.0 0 (`|MakeArray` 1.0 1.0 0.0 0.0 0.0 0.0 0.0 :!type "Float (single-precision)") (`|MakeArray` 450.0 -325.0 217.0 3.14 0.0 1.57 0.0 :!type "Float (single-precision)")) (make `NrcCmd` 1 100.0 30.0 30.0 1.0 0 (`|MakeArray` 1.0 1.0 0.0 0.0 0.0 0.0 0.0 :!type "Float (single-precision)") (`|MakeArray` 700.0 -325.0 350.0 3.14 0.0 1.57 0.0 :!type "Float (single-precision)"))) 2
      (:`then`
        (`KismetSystemLibrary.PrintString` "发送连续运动队列"))
      (:`OnSuccess`
        (`KismetSystemLibrary.PrintString` "发送连续运动队列 success")))))

(event `Key|Eight`
  (params (Key :type "Key Structure")))

(event `Key|Nine`
  (params (Key :type "Key Structure")))

(event `Key|Zero`
  (params (Key :type "Key Structure")))

(fn `UserConstructionScript`)